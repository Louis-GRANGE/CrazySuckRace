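; Player-drivable Chaos wheeled muscle car with axis-driven throttle, brake and steering, plus extra angular damping while airborne.
; A looping timer checks rear wheels for slip or skid, spawning, updating and detaching per-wheel Niagara smoke and tire mark emitters.
; Skid-based counter-steer and delayed ESP logic sets steering and traction variables in a custom event, but the CounterSteerSensivity function called on Tick is empty.
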(event Custom|Timer
  (CallFunction|DetectDrift))

(event Custom|CustomEvent
  ;[1 1 1] Counter Steer Sensivity
  (CallFunction|DetectRightSkidding)
  (CallFunction|DetectLefttSkidding)
  (if (Variables|Default|GetLeftSkidding)
    (if (Variables|Default|GetRightSkidding)
      (Utilities|FlowControl|Delay 1.5)
      (Variables|Default|SetSteeringSensivity 1.0)
      (Variables|Default|SetTractionMultiplier 1.0)
      (Variables|Default|SetCounterSteering false)
      (Variables|Default|SetTractionControlActive false)
      (else
        (Variables|Default|SetSteeringSensivity 3.0)
        (Variables|Default|SetCounterSteering true)
        (if (Variables|Default|GetESP%20On)
          (Utilities|FlowControl|Delay 0.5)
          (Variables|Default|SetTractionMultiplier 4.0)
          (Variables|Default|SetTractionControlActive true))))
    (else
      (Variables|Default|SetSteeringSensivity 3.0)
      (Variables|Default|SetCounterSteering true)
      (if (Variables|Default|GetESP%20On)
        (Utilities|FlowControl|Delay 0.5)
        (Variables|Default|SetTractionMultiplier 4.0)
        (Variables|Default|SetTractionControlActive true)))))

(event Custom|Detect%20Leftt%20Skidding)

(event Custom|Detect%20Leftt%20Skidiing
  ;[1 1 1] Detect Leftt Skidding
  (if (> (.SkidMagnitude (Class|ChaosWheeledVehicleMovementComponent|BreakWheelStatus (Class|ChaosWheeledVehicleMovementComponent|GetWheelState (Variables|Default|GetChaos%20Wheeled%20Vehicle%20Movement%20Component) 3))) -4e+02)
    (Variables|Default|SetLeftSkidding true)
    (else
      (Variables|Default|SetLeftSkidding false))))

(event Custom|Detect%20Right%20Skidding
  ;[1 1 1] Detect Right Skidding
  (if (< (.SkidMagnitude (Class|ChaosWheeledVehicleMovementComponent|BreakWheelStatus (Class|ChaosWheeledVehicleMovementComponent|GetWheelState (Variables|Default|GetChaos%20Wheeled%20Vehicle%20Movement%20Component) 3))) 4e+02)
    (Variables|Default|SetRightSkidding true)
    (else
      (Variables|Default|SetRightSkidding false))))

(event EventTick
  (params (DeltaSeconds :type Float%20%28single-precision%29))
  ;[1 1 1] Movement component setup
  (CallFunction|CounterSteerSensivity)
  (Class|PrimitiveComponent|SetAngularDamping (Variables|Character|GetMesh) (Math|Float|SelectFloat 0.0 3.0 (AI|Components|NavMovement|IsMovingonGround (Variables|Default|GetChaos%20Wheeled%20Vehicle%20Movement%20Component)))) ; Damps rotation when in air
)

(event EventBeginPlay
  ;[1 1 1] Movement component setup
  (Utilities|Time|SetTimerbyEvent (delegate Custom|Timer) 0.2 true)
  (bind _aschaos_wheeled_vehicle_movement_component (Utilities|Casting|CastToChaosWheeledVehicleMovementComponent (Variables|Default|GetVehicleMovementComponent)))
  (Variables|Default|SetChaos%20Wheeled%20Vehicle%20Movement%20Component _aschaos_wheeled_vehicle_movement_component))

(event Input|AxisEvents|InputAxisMoveRight
  (params (AxisValue :type Float%20%28single-precision%29))
  (Class|ChaosVehicleMovementComponent|SetSteeringInput (Variables|Default|GetVehicleMovementComponent) AxisValue))

(event Input|AxisEvents|InputAxisMoveForward
  (params (AxisValue :type Float%20%28single-precision%29))
  (bind _vehiclemovementcomponent (Variables|Default|GetVehicleMovementComponent))
  (bind _vehiclemovementcomponent_2 (Variables|Default|GetVehicleMovementComponent))
  (if (>= AxisValue 0.0)
    (Class|ChaosVehicleMovementComponent|SetThrottleInput _vehiclemovementcomponent AxisValue)
    (Class|ChaosVehicleMovementComponent|SetBrakeInput _vehiclemovementcomponent 0.0)
    (else
      (Class|ChaosVehicleMovementComponent|SetBrakeInput _vehiclemovementcomponent_2 (* AxisValue -1.0))
      (Class|ChaosVehicleMovementComponent|SetThrottleInput _vehiclemovementcomponent_2 0.0))))

(fn ConstructionScript)

(fn VehiculeInputs
  (bind _vehiclemovementcomponent (Variables|Default|GetVehicleMovementComponent))
  (Class|ChaosVehicleMovementComponent|SetThrottleInput _vehiclemovementcomponent (Input|AxisValues|GetThrottle_Input))
  (Class|ChaosVehicleMovementComponent|SetBrakeInput _vehiclemovementcomponent (Input|AxisValues|GetBrake_Input))
  (Class|ChaosVehicleMovementComponent|SetSteeringInput _vehiclemovementcomponent (Input|AxisValues|GetSteering_Input))
  (Class|ChaosVehicleMovementComponent|SetHandbrakeInput _vehiclemovementcomponent (== (Input|AxisValues|GetHandBrake_Input) 1.0)))

(fn CameraInput
  (Transformation|AddRelativeRotation (Variables|Default|GetSpringArm) (Math|Rotator|MakeRotator 0.0 (Input|AxisValues|GetLookRight) (Input|AxisValues|GetLookRight)) false false))

(fn CounterSteerSensivity)

(fn DetectDrift
  (bind _chaos_wheeled_vehicle_movement_component (Variables|Default|GetChaos%20Wheeled%20Vehicle%20Movement%20Component))
  (for (_array_element _array_index) (Variables|/Script/ChaosVehicles.ChaosWheeledVehicleMovementComponent|GetWheels _chaos_wheeled_vehicle_movement_component)
    (if (Math|Integer|InRange(Integer) _array_index 2 3)
      (if (and (not (Class|ChaosVehicleWheel|IsinAir _array_element)) (or (.bIsSlipping (Class|ChaosWheeledVehicleMovementComponent|BreakWheelStatus (Class|ChaosWheeledVehicleMovementComponent|GetWheelState _chaos_wheeled_vehicle_movement_component _array_index))) (.bIsSkidding (Class|ChaosWheeledVehicleMovementComponent|BreakWheelStatus (Class|ChaosWheeledVehicleMovementComponent|GetWheelState _chaos_wheeled_vehicle_movement_component _array_index)))))
        (if (== (Utilities|Array|Get(acopy) (Variables|Default|GetDrift%20Emmiters) _array_index) 0)
          (|Driftingbutnoemmiterfoundforthiswheel_2 _array_index (.SlipMagnitude (Class|ChaosWheeledVehicleMovementComponent|BreakWheelStatus (Class|ChaosWheeledVehicleMovementComponent|GetWheelState _chaos_wheeled_vehicle_movement_component _array_index))))
          (else
            (|Driftingandemmiteralreadyexistforthiswheel_2 (Utilities|Array|Get(acopy) (Variables|Default|GetDrift%20Emmiters) _array_index) (.SlipMagnitude (Class|ChaosWheeledVehicleMovementComponent|BreakWheelStatus (Class|ChaosWheeledVehicleMovementComponent|GetWheelState _chaos_wheeled_vehicle_movement_component _array_index))) (.SkidMagnitude (Class|ChaosWheeledVehicleMovementComponent|BreakWheelStatus (Class|ChaosWheeledVehicleMovementComponent|GetWheelState _chaos_wheeled_vehicle_movement_component _array_index))))))
        (else
          (|Wheelisinairorjustnotdrifting_2 _array_index))))))