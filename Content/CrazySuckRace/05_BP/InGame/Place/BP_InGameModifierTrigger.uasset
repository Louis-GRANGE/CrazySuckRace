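; Trigger volume that applies a configurable modifier to muscle cars entering its box, passing the trigger's forward vector as direction.
; Timer Based triggers go unavailable, then either self-destroy after a short delay or schedule an availability reset.
; Presence triggers remove the added modifier type on exit.
; Tick also restores availability every frame, so the timed cooldown does not persist between frames.
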(event OnComponentBeginOverlap(Box)
  (params (OverlappedComponent :type Primitive%20Component%20Object%20Reference) (OtherActor :type Actor%20Object%20Reference) (OtherComp :type Primitive%20Component%20Object%20Reference) (OtherBodyIndex :type Integer) (bFromSweep :type Boolean) (SweepResult :type Hit%20Result%20Structure%20%28by%20ref%29))
  (bind _asbp_muscle_car_v3 (Utilities|Casting|CastToBP_MuscleCar_V3 OtherActor))
  (if (Variables|Default|GetbIsAvailable)
    (bind _out_added_modifier (Default|AddModifier _asbp_muscle_car_v3 (Variables|Default|GetModifierToApply) (Math|Vector|GetForwardVector (Variables|Default|GetDefaultSceneRoot))))
    (Variables|Default|SetOut%20Added%20Modifier _out_added_modifier)
    (switch Utilities|FlowControl|Switch|SwitchonE_ModifierTriggerType (Variables|Default|GetModifierTriggerType)
      (:NewEnumerator0
        (Variables|Default|SetbIsAvailable false)
        (if (Variables|Default|GetbAutoDestroy)
          (Utilities|FlowControl|Delay 0.2)
          (Actor|DestroyActor)
          (else
            (Utilities|Time|SetTimerbyEvent (delegate Custom|ResetAvailability) (Variables|Default|GetResetTime))))))))

(event OnComponentEndOverlap(Box)
  (params (OverlappedComponent :type Primitive%20Component%20Object%20Reference) (OtherActor :type Actor%20Object%20Reference) (OtherComp :type Primitive%20Component%20Object%20Reference) (OtherBodyIndex :type Integer))
  (bind _asbp_muscle_car_v3 (Utilities|Casting|CastToBP_MuscleCar_V3 OtherActor))
  (if (Variables|Default|GetbIsAvailable)
    (switch Utilities|FlowControl|Switch|SwitchonE_ModifierTriggerType (Variables|Default|GetModifierTriggerType)
      (:NewEnumerator1
        (Default|RemoveModifier _asbp_muscle_car_v3 (Variables|/Game/CrazySuckRace/05_BP/Modifiers/BP_BaseModifier.BP_BaseModifier_C|GetModifierType (Variables|Default|GetOut%20Added%20Modifier)))))))

(event Custom|ResetAvailability
  (Variables|Default|SetbIsAvailable true))

(event EventBeginPlay
  (|CallParentFunction) ; This node is disabled and will not be called.\nDrag off pins to build functionality.
)

(event Collision|EventActorBeginOverlap
  (params (OtherActor :type Actor%20Object%20Reference)))

(event EventTick
  (params (DeltaSeconds :type Float%20%28single-precision%29))
  (|CallParentFunction DeltaSeconds)
  (Variables|Default|SetbIsAvailable true))

(fn ConstructionScript
  (|CallParentFunction))