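; BP_PartToPlace is a selectable part for placement in CrazySuckRace, broadcasting OnSelected with itself on a primary mouse press.
; It caches its primitive components at BeginPlay and toggles their custom depth on cursor hover for highlighting.
; SetUseMask switches the UseDesapear material parameter on its static meshes.
; Mouse-trace grid-snap movement and debug drawing remain as unconnected leftovers, so the actor does not move itself.
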(event EventBeginPlay
  (Variables|Default|SetPrimitivesComponents (Actor|GetComponentsByClass "/Script/Engine.PrimitiveComponent")))

(event Collision|EventActorBeginOverlap
  (params (OtherActor :type Actor%20Object%20Reference)))

(event EventTick
  (params (DeltaSeconds :type Float%20%28single-precision%29)))

(event EventOnPrimaryMousePressed
  (Default|Call+OnSelected self))

(event EventOnBeginCursorHover
  (CallFunction|SetAllRenderCustomDepth true))

(event EventOnEndCursorHover
  (CallFunction|SetAllRenderCustomDepth false))

(fn ConstructionScript)

(fn SetAllRenderCustomDepth
  (params (UseRenderCustomDepth :type Boolean))
  (for _array_element (Variables|Default|GetPrimitivesComponents)
    (Rendering|SetRenderCustomDepth _array_element UseRenderCustomDepth)))

(fn SetUseMask
  (params (Use? :type Boolean))
  (for _array_element (Variables|Default|GetPrimitivesComponents)
    (bind _asstatic_mesh_component (Utilities|Casting|CastToStaticMeshComponent _array_element))
    (Rendering|Material|SetScalarParameterValueonMaterials _asstatic_mesh_component "UseDesapear" (select Use? 1.0 0.0))))