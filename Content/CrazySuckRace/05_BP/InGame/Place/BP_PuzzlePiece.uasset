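; Collectible puzzle piece for Crazy Suck Race that spins around its yaw axis each tick at the Rotating rate.
; When a BP_MuscleCar_V3 overlaps its capsule, it calls GainOnePiece on that car's PC_InGame-CrazySuckRace controller and destroys itself.
; It binds to the lobby game state's OnAllPlayerFinishRace on BeginPlay so leftover pieces are removed once the race is over.
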(event OnComponentBeginOverlap(Capsule)
  (params (OverlappedComponent :type Primitive%20Component%20Object%20Reference) (OtherActor :type Actor%20Object%20Reference) (OtherComp :type Primitive%20Component%20Object%20Reference) (OtherBodyIndex :type Integer) (bFromSweep :type Boolean) (SweepResult :type Hit%20Result%20Structure%20%28by%20ref%29))
  (bind _asbp_muscle_car_v3 (Utilities|Casting|CastToBP_MuscleCar_V3 OtherActor))
  (bind _aspc_in_game__crazy_suck_race (Utilities|Casting|CastToPC_InGame-CrazySuckRace (Pawn|GetController _asbp_muscle_car_v3)))
  (Default|GainOnePiece _aspc_in_game__crazy_suck_race)
  (Actor|DestroyActor))

(event Custom|DestroyOnFinishRace
  (Actor|DestroyActor))

(event EventBeginPlay
  (EventDispatchers|BindEventto+OnAllPlayerFinishRace (CallFunction|GetGSLobby-CrazySuckRace) (EventDispatchers|CreateEvent :!event Custom|DestroyOnFinishRace)))

(event Collision|EventActorBeginOverlap
  (params (OtherActor :type Actor%20Object%20Reference)))

(event EventTick
  (params (DeltaSeconds :type Float%20%28single-precision%29))
  (Transformation|AddActorLocalRotation (Math|Rotator|MakeRotator 0.0 0.0 (* DeltaSeconds (Variables|Default|Getrotating))) false false))

(fn ConstructionScript)