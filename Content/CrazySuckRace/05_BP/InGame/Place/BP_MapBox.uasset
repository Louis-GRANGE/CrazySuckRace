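; BP_MapBox is a map area actor that scatters puzzle pieces for Crazy Suck Race.
; On the server, BeginPlay binds GeneratePuzzlePieces to the lobby game state's end-of-construct-phase event.
; That event spawns AmountOfPuzzlePieces BP_PuzzlePiece actors at random XY points within the static mesh's bounds, at a fixed height above the bounds' center.
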(event Custom|GeneratePuzzlePieces
  (bind _staticmesh (Variables|Default|GetStaticMesh))
  (bind (_origin _boxextent) (Collision|GetComponentBounds _staticmesh))
  (bind _returnvalue (Math|Random|RandomPointinBoundingBox (Math|Vector|MakeVector (.x _origin) (.y _origin) 0.0) (Math|Vector|MakeVector (.x _boxextent) (.y _boxextent) 0.0)))
  (for _index (range 1 (Variables|Default|GetAmountOfPuzzlePieces))
    (Game|SpawnActorfromClass "/Game/CrazySuckRace/05_BP/InGame/Place/BP_PuzzlePiece.BP_PuzzlePiece_C" (Math|Transform|MakeTransform (Math|Vector|MakeVector (.x _returnvalue) (.y _returnvalue) (+ (.z _origin) 2e+02)) "0, 0, 0" "1.000000,1.000000,1.000000") "Undefined" 0 0)))

(event EventBeginPlay
  (Networking|SwitchHasAuthority
    (:Authority
      (EventDispatchers|BindEventto+OnEndPhaseConstruct (CallFunction|GetGSLobby-CrazySuckRace) (delegate Custom|GeneratePuzzlePieces)))))

(event Collision|EventActorBeginOverlap
  (params (OtherActor :type Actor%20Object%20Reference)))

(event EventTick
  (params (DeltaSeconds :type Float%20%28single-precision%29)))

(fn ConstructionScript)