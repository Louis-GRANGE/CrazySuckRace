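; Construction-phase part spawner for CrazySuckRace that offers random placeable parts once all players finish a race.
; On authority, it binds to GameState events, spawns parts at the Box's child component locations, and destroys unplaced ones when construction ends.
; It fits a material parameter collection sphere mask to the Box bounds.
; Selection masking, grid-snapped mouse dragging and overlap repositioning are disconnected, leaving the selection handler empty.
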(event Custom|Evt_OnSelectPart
  (params (PartRef :type BP%20Part%20to%20Place%20Object%20Reference)))

(event Custom|GenerateAllPart
  (bind _box (Variables|Default|GetBox))
  (bind (_origin _boxextent _sphereradius) (Collision|GetComponentBounds _box))
  (Variables|Default|SetSphereComponent (Components|GetChildrenComponents (Variables|Default|GetBox) false))
  (for _index (range 0 (- (Variables|Default|GetNbPartToGenerate) 1))
    (bind _returnvalue (Game|SpawnActorfromClass (.OutItem (Utilities|Array|Random (Variables|Default|GetCanGeneratePart))) (Math|Transform|MakeTransform (Transformation|GetWorldLocation (Utilities|Array|Get(acopy) (Variables|Default|GetSphereComponent) _index)) "0, 0, 0" "1.000000,1.000000,1.000000") "Undefined" 0 0 false 0))
    (Utilities|Array|Add (Variables|Default|GetGeneratedPart) _returnvalue)
    (EventDispatchers|BindEventto+OnSelected _returnvalue (EventDispatchers|CreateEvent :!event Custom|Evt_OnSelectPart)))
  (bind _returnvalue_2 (Utilities|Time|SetTimerbyEvent (EventDispatchers|CreateEvent :!event Custom|CheckingLocation) 0.001 true))
  (Variables|Default|SetEvt_CheckingLocation _returnvalue_2)
  (Rendering|Material|SetScalarParameterValue "/Game/CrazySuckRace/04_Material/_ParameterCollection/MPC_PartSelection.MPC_PartSelection" "SphereMask-Radius" _sphereradius :!class /Script/Engine.KismetMaterialLibrary)
  (Rendering|Material|SetVectorParameterValue "/Game/CrazySuckRace/04_Material/_ParameterCollection/MPC_PartSelection.MPC_PartSelection" "SphereMask-Location" (Math|Conversions|ToLinearColor(Vector) _origin) :!class /Script/Engine.KismetMaterialLibrary))

(event Custom|CheckingLocation
  (Utilities|Time|ClearandInvalidateTimerbyHandle (Variables|Default|GetEvt_CheckingLocation)))

(event Custom|EVt_OnAllPlayerFinishRace
  (CallFunction|GenerateAllPart))

(event Custom|SpawnClassOnServer
  (params (Class :type BP%20Part%20to%20Place%20Class%20Reference))
  (bind _returnvalue (Game|SpawnActorfromClass Class (Math|Transform|MakeTransform (Transformation|GetActorLocation) "0, 0, 0" "1.000000,1.000000,1.000000") "Undefined" 0 0 false 0))
  (Variables|Default|SetSelectedPart _returnvalue)
  (Networking|SetReplicates _returnvalue true)
  (Class|Actor|SetReplicateMovement _returnvalue true))

(event Custom|Evt_OnEndPhaseConstruction
  (bind _generatedpart (Variables|Default|GetGeneratedPart))
  (for _array_element _generatedpart
    (if (not (Variables|/Game/CrazySuckRace/05_BP/InGame/Place/BP_PartToPlace.BP_PartToPlace_C|GetIsPlaced _array_element))
      (Actor|DestroyActor _array_element)))
  (Utilities|Array|Clear _generatedpart))

(event EventBeginPlay
  (Networking|SwitchHasAuthority
    (:Authority
      (bind _aspc_in_game__crazy_suck_race (Utilities|Casting|CastToPC_InGame-CrazySuckRace (Game|GetPlayerController 0)))
      (Variables|Default|SetPCRef _aspc_in_game__crazy_suck_race)
      (CallFunction|EVtonAllPlayerFinishRace)
      (bind _asgs_lobby__crazy_suck_race (Utilities|Casting|CastToGS_Lobby-CrazySuckRace (Game|GetGameState)))
      (EventDispatchers|BindEventto+OnAllPlayerFinishRace _asgs_lobby__crazy_suck_race (EventDispatchers|CreateEvent :!event Custom|EVt_OnAllPlayerFinishRace))
      (EventDispatchers|BindEventto+OnEndPhaseConstruct _asgs_lobby__crazy_suck_race (EventDispatchers|CreateEvent :!event Custom|Evt_OnEndPhaseConstruction)))))

(event Collision|EventActorBeginOverlap
  (params (OtherActor :type Actor%20Object%20Reference)))

(event EventTick
  (params (DeltaSeconds :type Float%20%28single-precision%29)))

(fn ConstructionScript)

(fn CheckifPartIsinOthersParts
  (params (PartRef :type BP%20Part%20to%20Place%20Object%20Reference))
  (bind _box (Variables|Default|GetBox))
  (bind (_origin _boxextent) (Collision|GetComponentBounds _box))
  (for _array_element (Variables|Default|GetGeneratedPart)
    (if (Collision|IsOverlappingActor _array_element PartRef :!class /Script/Engine.Actor)
      (Transformation|SetActorLocation PartRef (Math|Random|RandomPointinBoundingBox _origin _boxextent) false false)
      (return true)))
  (return false))