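; Placeable track part for CrazySuckRace that carries a checkpoint as a child actor and registers it with the custom map when placed.
; On place, it adds its BP_CheckPoint to the list in BP_CustomCheckPointsMap, then sets the lobby game state's checkpoint-to-validate count to that list's length.
; It also prints the count for debugging; the server placement event only calls the parent.
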(event EventBeginPlay
  (|CallParentFunction) ; This node is disabled and will not be called.\nDrag off pins to build functionality.
)

(event Collision|EventActorBeginOverlap
  (params (OtherActor :type Actor%20Object%20Reference)))

(event EventTick
  (params (DeltaSeconds :type Float%20%28single-precision%29))
  (|CallParentFunction DeltaSeconds) ; This node is disabled and will not be called.\nDrag off pins to build functionality.
)

(event EventOnPlace-Server
  (params (TeamColor :type Linear%20Color%20Structure))
  ;[1 1 1] TO CHECK
  (|CallParentFunction TeamColor))

(event EventOnPlace
  (params (TeamColor :type Linear%20Color%20Structure))
  ;[1 1 1] TO CHECK
  (|CallParentFunction TeamColor)
  (bind _returnvalue (Actor|GetActorOfClass "/Game/CrazySuckRace/05_BP/InGame/BP_CustomCheckPointsMap.BP_CustomCheckPointsMap_C"))
  (bind _asbp_check_point (Utilities|Casting|CastToBP_CheckPoint (Variables|/Script/Engine.ChildActorComponent|GetChildActor (Variables|Default|GetChildActor))))
  (Utilities|Array|Add (Variables|/Game/CrazySuckRace/05_BP/InGame/BP_CustomCheckPointsMap.BP_CustomCheckPointsMap_C|GetAllCheckPoints _returnvalue) _asbp_check_point)
  (bind _output_get (Variables|/Game/CrazySuckRace/05_BP/Lobby/GS_Lobby-CrazySuckRace.GS_Lobby-CrazySuckRace_C|SetNbCheckPointToValidate (CallFunction|GetGSLobby-CrazySuckRace) (Utilities|Array|Length (Variables|/Game/CrazySuckRace/05_BP/InGame/BP_CustomCheckPointsMap.BP_CustomCheckPointsMap_C|GetAllCheckPoints _returnvalue))))
  (Development|PrintString (Utilities|String|Append "Len: " (Utilities|String|ToString(Integer) _output_get)) true true "(R=0.440394,G=1.000000,B=0.000000,A=1.000000)" 2e+02))

(fn ConstructionScript
  (|CallParentFunction))