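; BP_PartToPlace-Road is a road part for placement that flags when it overlaps another road part.
; Begin overlap with the same class sets IsOverlapingWrongActor and binds a handler to the other part's OnActorEndOverlap.
; That handler clears the flag whenever the other part ends any overlap, without checking which actor left.
; Both transitions print debug strings, and construction only calls the parent.
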(event Custom|OnActorEndOverlap_Event
  (params (OverlappedActor :type Actor%20Object%20Reference) (OtherActor :type Actor%20Object%20Reference))
  (Development|PrintString "OVERLAP FALSE" true true "(R=0.000000,G=0.660000,B=1.000000,A=1.000000)" 2e+01)
  (Variables|Default|SetisOverlapingWrongActor? false))

(event EventBeginPlay
  (|CallParentFunction) ; This node is disabled and will not be called.\nDrag off pins to build functionality.
)

(event Collision|EventActorBeginOverlap
  (params (OtherActor :type Actor%20Object%20Reference))
  (bind _asbp_part_to_place__road (Utilities|Casting|CastToBP_PartToPlace-Road OtherActor))
  (Variables|Default|SetisOverlapingWrongActor? true)
  (Development|PrintString "OVERLAP TRUE" true true "(R=0.000000,G=0.660000,B=1.000000,A=1.000000)" 2e+01)
  (EventDispatchers|BindEventtoOnActorEndOverlap _asbp_part_to_place__road (delegate Custom|OnActorEndOverlap_Event)))

(event EventTick
  (params (DeltaSeconds :type Float%20%28single-precision%29))
  (|CallParentFunction DeltaSeconds) ; This node is disabled and will not be called.\nDrag off pins to build functionality.
)

(fn ConstructionScript
  (|CallParentFunction))