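; In-game GameMode for CrazySuckRace that tracks players arriving after travel and handles server travel to levels.
; On BeginPlay and after each PostLogin, it compares the player count with the GameInstance's expected count, then notifies the game state once all have arrived.
; Joins and logouts are relayed through the lobby game state's multicast calls after short delays.
; TravelByRef and TravelByName wrap ServerTravel for level references or names.
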(event Custom|OnServerJoinGame
  (bind _returnvalue (Class|GameModeBase|GetNumPlayers))
  (bind _asgi_crazy_suck_race (Utilities|Casting|CastToGI_CrazySuckRace (Game|GetGameInstance)))
  (if (== (Variables|/Game/CrazySuckRace/05_BP/GI_CrazySuckRace.GI_CrazySuckRace_C|GetNbPlayerInServer _asgi_crazy_suck_race) _returnvalue)
    (Utilities|FlowControl|Delay 0.5)
    (Default|OnAllPlayerTravels (CallFunction|GetGSLobby-CrazySuckRace))))

(event Custom|TravelByName
  (params (InURL :type String))
  (Class|AdvancedSessionsLibrary|ServerTravel InURL false false)
  (Development|PrintString "No \".\" in your GAME LEVEL thx" false true "(R=1.000000,G=0.000000,B=0.047184,A=1.000000)"))

(event Custom|TravelByRef
  (params (Level :type World%20Soft%20Object%20Reference))
  (Class|AdvancedSessionsLibrary|ServerTravel (.LeftS (Utilities|String|Split (Utilities|ToString(SoftObjectReference) Level) ".")) false false)
  (Development|PrintString "No \".\" in your GAME LEVEL thx" false true "(R=1.000000,G=0.000000,B=0.047184,A=1.000000)"))

(event EventBeginPlay
  (CallFunction|OnServerJoinGame))

(event EventTick
  (params (DeltaSeconds :type Float%20%28single-precision%29)))

(event EventOnLogout
  (params (ExitingController :type Controller%20Object%20Reference))
  (bind _asps_crazy_suck_race (Utilities|Casting|CastToPS_CrazySuckRace (Variables|/Script/Engine.Controller|GetPlayerState ExitingController)))
  (Utilities|FlowControl|Delay 1.0)
  (Default|CallonPlayerLeave-Muilticast (CallFunction|GetGSLobby-CrazySuckRace) _asps_crazy_suck_race))

(event EventPostLogin
  (params (NewPlayer :type Player%20Controller%20Object%20Reference))
  (bind _asps_crazy_suck_race (Utilities|Casting|CastToPS_CrazySuckRace (Variables|/Script/Engine.Controller|GetPlayerState NewPlayer)))
  (Utilities|FlowControl|Delay 1.0)
  (Default|CallonPlayerJoin-Multicast (CallFunction|GetGSLobby-CrazySuckRace) _asps_crazy_suck_race)
  (bind _returnvalue (Class|GameModeBase|GetNumPlayers))
  (bind _asgi_crazy_suck_race (Utilities|Casting|CastToGI_CrazySuckRace (Game|GetGameInstance)))
  (if (== (Variables|/Game/CrazySuckRace/05_BP/GI_CrazySuckRace.GI_CrazySuckRace_C|GetNbPlayerInServer _asgi_crazy_suck_race) _returnvalue)
    (Utilities|FlowControl|Delay 0.5)
    (Default|OnAllPlayerTravels (CallFunction|GetGSLobby-CrazySuckRace))))

(fn ConstructionScript)