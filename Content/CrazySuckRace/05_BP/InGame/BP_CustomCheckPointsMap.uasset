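; Custom map actor for CrazySuckRace that places the race checkpoints and spawns players' cars.
; On the server, after a short delay, it spawns BP_CheckPoint actors at randomly picked, non-repeating child placements, with the count set by the lobby's MapSize.
; It also binds to the game state's end-of-construct-phase event.
; Evt_SpawnCarsToRace spawns muscle cars at one random checkpoint's spawn points and possesses them with player controllers, starting at index 1.
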(event Custom|Evt_SpawnCarsToRace
  (bind _asgm_in_game__crazy_suck_race (Utilities|Casting|CastToGM_InGame-CrazySuckRace (Game|GetGameMode)))
  (bind _returnvalue (Class|GameModeBase|GetNumPlayers _asgm_in_game__crazy_suck_race))
  (bind _outitem (CallFunction|GetRandomCheckPoint))
  (for _index (range 0 (- _returnvalue 1))
    (bind _returnvalue_2 (Game|SpawnActorfromClass "/Game/CrazySuckRace/05_BP/VoitureMuscleCar/V3_Nicolas/BP_MuscleCar_V3.BP_MuscleCar_V3_C" (Math|Transform|MakeTransform (+ (.location (Transformation|GetWorldTransform (Utilities|Array|Get(acopy) (Variables|/Game/CrazySuckRace/05_BP/InGame/BP_CheckPoint.BP_CheckPoint_C|GetAllSpawnPoints _outitem) _index))) "0,0,100.000000") (.rotation (Transformation|GetWorldTransform (Utilities|Array|Get(acopy) (Variables|/Game/CrazySuckRace/05_BP/InGame/BP_CheckPoint.BP_CheckPoint_C|GetAllSpawnPoints _outitem) _index))) (.scale (Transformation|GetWorldTransform (Utilities|Array|Get(acopy) (Variables|/Game/CrazySuckRace/05_BP/InGame/BP_CheckPoint.BP_CheckPoint_C|GetAllSpawnPoints _outitem) _index)))) "AlwaysSpawn" (Game|GetPlayerController (+ _index 1)) 0))
    (Pawn|Possess (Game|GetPlayerController (+ _index 1)) _returnvalue_2)))

(event EventBeginPlay
  (Networking|SwitchHasAuthority
    (:Authority
      (Utilities|FlowControl|Delay 0.5)
      (CallFunction|SpawnAllCheckPoints)
      (EventDispatchers|BindEventto+OnEndPhaseConstruct (CallFunction|GetGSLobby-CrazySuckRace) (EventDispatchers|CreateEvent :!event Custom|Evt_SpawnCarsToRace)))))

(event Collision|EventActorBeginOverlap
  (params (OtherActor :type Actor%20Object%20Reference)))

(event EventTick
  (params (DeltaSeconds :type Float%20%28single-precision%29)))

(fn ConstructionScript)

(fn SpawnAllCheckPoints
  (CallFunction|DestroyCheckPoints)
  (bind _randomcheckpoints (CallFunction|GetRandomInitCheckPoints (Components|GetChildrenComponents (Variables|Default|GetCheckPoints) false)))
  (for _array_element _randomcheckpoints
    (bind _returnvalue (Game|SpawnActorfromClass "/Game/CrazySuckRace/05_BP/InGame/BP_CheckPoint.BP_CheckPoint_C" (Transformation|GetWorldTransform _array_element) "Undefined" 0 0))
    (Utilities|Array|Add (Variables|Default|GetAllCheckPoints) _returnvalue)))

(fn DestroyCheckPoints
  (bind _allcheckpoints (Variables|Default|GetAllCheckPoints))
  (for _array_element _allcheckpoints
    (Actor|DestroyActor _array_element))
  (Utilities|Array|Clear _allcheckpoints))

(fn GetRandomCheckPoint
  (return (.OutItem (Utilities|Array|Random (Variables|Default|GetAllCheckPoints)))))

(fn GetRandomInitCheckPoints
  (params (CheckPointsPlacements :type Array%20of%20Scene%20Component%20Object%20References))
  (bind _return_value (CallFunction|GetGSLobby-CrazySuckRace))
  (bind _gamesettings (Variables|/Game/CrazySuckRace/05_BP/Lobby/GS_Lobby-CrazySuckRace.GS_Lobby-CrazySuckRace_C|GetGameSettings _return_value))
  (bind _mapsize (Utilities|Struct|BreakS_GameSettings _gamesettings))
  (bind _returnvalue (Utilities|Select :Index _mapsize :NewEnumerator0 2 :NewEnumerator1 3 :NewEnumerator2 4))
  (LocalVariables|SetTmp CheckPointsPlacements)
  (Development|PrintString (Utilities|String|Append (Utilities|String|EnumtoString _mapsize) " " (Utilities|String|ToString(Integer) _returnvalue)) true true "(R=1.000000,G=0.000000,B=0.070010,A=1.000000)" 3e+01)
  (for _index (range 1 _returnvalue)
    (bind _output_get (LocalVariables|SetRefRandom (.OutItem (Utilities|Array|Random (LocalVariables|GetTmp)))))
    (Utilities|Array|Add (LocalVariables|GetCheckPointsToReturn) _output_get)
    (Utilities|Array|RemoveItem (LocalVariables|GetTmp) _output_get))
  (return (LocalVariables|GetCheckPointsToReturn)))