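; BP_EngineSlowModifier is a car modifier that changes the engine torque of the BP_MuscleCar_V3 it is attached to, named as a slowdown.
; On BeginPlay it sets its modifier type, runs the parent logic, then applies the car's torque scaled by BoostMultiplier as the movement component's max engine torque.
; DeactivateModifier has the car reset its torque.
; Tick only prints an "attached" debug string.
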(event EventBeginPlay
  (Variables|Default|SetModifierType "NewEnumerator0")
  (|CallParentFunction)
  (bind _asbp_muscle_car_v3 (Utilities|Casting|CastToBP_MuscleCar_V3 (Components|GetOwner)))
  (bind _output_get (Variables|Default|SetOwner _asbp_muscle_car_v3))
  (bind _outtorque (Default|GetEngineTorque _output_get))
  (bind _output_get_2 (Variables|Default|SetTorqueBeforeBoost _outtorque))
  (bind _output_get_3 (Variables|Default|SetBoostTorque (* _output_get_2 (Variables|Default|GetBoostMultiplier))))
  (Class|ChaosWheeledVehicleMovementComponent|SetMaxEngineTorque (Variables|/Game/CrazySuckRace/05_BP/VoitureMuscleCar/V3_Nicolas/BP_MuscleCar_V3.BP_MuscleCar_V3_C|GetChaos%20Wheeled%20Vehicle%20Movement%20Component _output_get) _output_get_3))

(event EventTick
  (params (DeltaSeconds :type Float%20%28single-precision%29))
  (Development|PrintString "attached" true true "(R=0.000000,G=0.660000,B=1.000000,A=1.000000)" 2.0 "attached"))

(fn DeactivateModifier
  (Default|ResetEngineTorque (Variables|Default|GetOwner)))