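; Impact modifier component or actor that knocks a BP_MuscleCar_V3 with a one-off physics impulse.
; BeginPlay sets a short auto-destroy delay and the modifier type before running the parent logic.
; The push happens in DeactivateModifier, after the parent call, by applying ModifierDirection times ImpulseForce to the owning car's mesh as a velocity change, so mass is ignored.
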(event EventBeginPlay
  (Variables|Default|SetAutoDestroyDelay 0.1)
  (Variables|Default|SetModifierType "NewEnumerator3")
  (|CallParentFunction))

(fn DeactivateModifier
  (|CallParentFunction)
  (bind _asbp_muscle_car_v3 (Utilities|Casting|CastToBP_MuscleCar_V3 (Components|GetOwner)))
  (Physics|AddImpulse (Variables|/Script/ChaosVehicles.WheeledVehiclePawn|GetMesh _asbp_muscle_car_v3) (* (Variables|Default|GetModifierDirection) (Variables|Default|GetImpulseForce)) "None" true))