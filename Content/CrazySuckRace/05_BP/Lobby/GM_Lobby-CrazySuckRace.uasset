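; Lobby game mode for CrazySuckRace that tracks players joining and leaving and moves the session to a level.
; Login and logout cast the controller's PlayerState to PS_CrazySuckRace and forward it to the lobby GameState's join and leave calls.
; The Travel event converts the given level to a string, keeps the part before the first "." and passes it to ServerTravel.
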(event Custom|Travel
  (params (Level :type World%20Soft%20Object%20Reference))
  (Class|AdvancedSessionsLibrary|ServerTravel (.LeftS (Utilities|String|Split (Utilities|ToString(SoftObjectReference) Level) ".")) false false)
  (Development|PrintString "No \".\" in your GAME LEVEL thx" false true "(R=1.000000,G=0.000000,B=0.047184,A=1.000000)"))

(event EventBeginPlay)

(event EventTick
  (params (DeltaSeconds :type Float%20%28single-precision%29)))

(event EventPostLogin
  (params (NewPlayer :type Player%20Controller%20Object%20Reference))
  (bind _asps_crazy_suck_race (Utilities|Casting|CastToPS_CrazySuckRace (Variables|/Script/Engine.Controller|GetPlayerState NewPlayer)))
  (Default|Call+OnPlayerJoin (CallFunction|GetGSLobby-CrazySuckRace) _asps_crazy_suck_race))

(event EventOnLogout
  (params (ExitingController :type Controller%20Object%20Reference))
  (bind _asps_crazy_suck_race (Utilities|Casting|CastToPS_CrazySuckRace (Variables|/Script/Engine.Controller|GetPlayerState ExitingController)))
  (Default|Call+OnPlayerLeave (CallFunction|GetGSLobby-CrazySuckRace) _asps_crazy_suck_race))

(fn ConstructionScript)