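; Lobby player controller for CrazySuckRace that gives the local player a random team color on join.
; On BeginPlay, the local controller asks the lobby GameState for an untaken random color.
; It passes that color through a server event to the CrazySuckRace PlayerState and also stores it in the GameInstance.
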(event Custom|SetTeamColor-Server
  (params (TeamColor :type Linear%20Color%20Structure))
  (bind _asps_crazy_suck_race (Utilities|Casting|CastToPS_CrazySuckRace (Variables|GetPlayerState)))
  (Default|SetTeamColor _asps_crazy_suck_race TeamColor))

(event EventBeginPlay
  (if (Pawn|IsLocalPlayerController)
    (bind _randomcolor (Default|GetUnTakedRandomColor (CallFunction|GetGSLobby-CrazySuckRace)))
    (CallFunction|SetTeamColor-Server _randomcolor)
    (bind _asgi_crazy_suck_race (Utilities|Casting|CastToGI_CrazySuckRace (Game|GetGameInstance)))
    (Variables|/Game/CrazySuckRace/05_BP/GI_CrazySuckRace.GI_CrazySuckRace_C|SetTeamColor _asgi_crazy_suck_race _randomcolor)))

(event EventTick
  (params (DeltaSeconds :type Float%20%28single-precision%29)))

(fn ConstructionScript)